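; Cannon turret actor that constantly turns to face the player and fires burst projectiles on a timer.
; FacePlayer interpolates rotation toward the player and re-calls itself through a tiny Delay instead of using Tick.
; Start_Timer runs Cannon_Shoot on a looping timer, which spawns the projectile, plays the shot sound and triggers the anim blueprint.
; End_Timer clears the timer and resets the shot count and active flag.
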(event Custom|FacePlayer
  (bind _returnvalue (Transformation|GetActorRotation))
  (bind _returnvalue_2 (Utilities|Time|GetWorldDeltaSeconds))
  (bind _returnvalue_3 (Transformation|GetActorLocation))
  (bind _as_bp_bowen_tpc (Variables|Default|GetAs%20BP%20Bowen%20TPC))
  (bind _returnvalue_4 (Transformation|GetActorLocation _as_bp_bowen_tpc))
  (bind _returnvalue_5 (Math|Rotator|FindLookatRotation _returnvalue_3 _returnvalue_4))
  (bind _returnvalue_6 (Math|Interpolation|RInterpTo _returnvalue _returnvalue_5 _returnvalue_2 2e+01))
  ;[1 1 1] Face Player
  (Transformation|SetActorRotation (Math|Rotator|MakeRotator (.roll _returnvalue_6) (.pitch _returnvalue_6) (.yaw _returnvalue_6)))
  (Utilities|FlowControl|Delay 0.001)
  (CallFunction|FacePlayer))

(event Custom|Cannon_Shoot
  (bind _scene (Variables|Default|GetScene))
  (bind _returnvalue (Transformation|GetWorldTransform _scene))
  ;[1 1 1] Shoot
  (Variables|Default|SetBullet%20Shot (+ (Variables|Default|GetBullet%20Shot) 1))
  (Game|SpawnActorfromClass "/Game/Robert/BP_BasePorjectileBurst.BP_BasePorjectileBurst_C" (Math|Transform|MakeTransform (.location _returnvalue) (.rotation _returnvalue) "1.000000,1.000000,1.000000") "Undefined" 0 5e+02 0)
  (Audio|PlaySoundatLocation "/Game/Robert/turretshot.turretshot" (.location _returnvalue) "0, 0, 0" 1.0 1.0 0.0 0 0 0 0)
  (Default|StartShooting (Variables|Default|GetAs%20ABP%20Cannon)))

(event Custom|Start_Timer
  (bind _returnvalue (Utilities|Time|SetTimerbyFunctionName 0 "Cannon_Shoot" 3.0 true))
  (Variables|Default|SetT_Cannon_Shoot _returnvalue)
  (Variables|Default|SetIsActive true))

(event Custom|End_Timer
  (Utilities|Time|ClearandInvalidateTimerbyHandle (Variables|Default|GetT_Cannon_Shoot))
  (Variables|Default|SetBullet%20Shot 0)
  (Variables|Default|SetIsActive false))

(event EventBeginPlay
  (bind _asbp_bowen_tpc (Utilities|Casting|CastToBP_Bowen_TPC (Game|GetPlayerCharacter 0)))
  (Variables|Default|SetAs%20BP%20Bowen%20TPC _asbp_bowen_tpc)
  (CallFunction|FacePlayer)
  (bind _asabp_cannon (Utilities|Casting|CastToABP_Cannon (Components|SkeletalMesh|GetAnimInstance (Variables|Default|GetSkeletalMesh))))
  (Variables|Default|SetAs%20ABP%20Cannon _asabp_cannon))

(event Collision|EventActorBeginOverlap
  (params (OtherActor :type Actor%20Object%20Reference)))

(event EventTick
  (params (DeltaSeconds :type Float%20%28single-precision%29)))

(fn ConstructionScript)