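; Burst projectile actor that applies damage on hit, with its movement speed set from a variable at construction.
; On hit it branches on a Hit flag: true damages the other actor and destroys the projectile, false awards player score through the game mode cached at BeginPlay.
; Both branches print debug text, and leftover health bar update logic is disconnected.
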(event OnComponentHit(Sphere1)
  (params (HitComponent :type Primitive%20Component%20Object%20Reference) (OtherActor :type Actor%20Object%20Reference) (OtherComp :type Primitive%20Component%20Object%20Reference) (NormalImpulse :type Vector :default "0, 0, 0") (Hit :type Hit%20Result%20Structure%20%28by%20ref%29)))

(event EventBeginPlay
  (bind _asbp_first_person_game_mode (Utilities|Casting|CastToBP_FirstPersonGameMode (Game|GetGameMode)))
  (Variables|Default|SetAs%20BP%20First%20Person%20Game%20Mode _asbp_first_person_game_mode))

(event Collision|EventActorBeginOverlap
  (params (OtherActor :type Actor%20Object%20Reference)))

(event EventTick
  (params (DeltaSeconds :type Float%20%28single-precision%29)))

(event Collision|EventHit
  (params (MyComp :type Primitive%20Component%20Object%20Reference) (Other :type Actor%20Object%20Reference) (OtherComp :type Primitive%20Component%20Object%20Reference) (bSelfMoved :type Boolean) (HitLocation :type Vector :default "0, 0, 0") (HitNormal :type Vector :default "0, 0, 0") (NormalImpulse :type Vector :default "0, 0, 0") (Hit :type Hit%20Result%20Structure%20%28by%20ref%29))
  (if (Variables|Default|GetHit?)
    (Variables|Default|SetHit? true)
    (Game|Damage|ApplyDamage Other 45.0 0 self)
    (Development|PrintString "Hit from projectile")
    (Actor|DestroyActor)
    (else
      (Variables|Default|SetHit? false)
      (Development|PrintString "Did not hit")
      (Default|AddPlayerScore (Variables|Default|GetAs%20BP%20First%20Person%20Game%20Mode) 20))))

(fn ConstructionScript
  (Variables|/Script/Engine.ProjectileMovementComponent|SetInitialSpeed (Variables|Default|GetProjectileMovement) (Variables|Default|GetIntial%20Speed)))