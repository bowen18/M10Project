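; BP_Spiketrap is a floor spike trap that damages the player character when they begin overlapping its Box component.
; When Activate is set, Tick replays the spike animation at random intervals, using a CanPlay flag and Delay to space each cycle.
; The overlap damage is a fixed amount and is independent of both the Activate flag and the animation state.
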(event OnComponentBeginOverlap(Box)
  (params (OverlappedComponent :type Primitive%20Component%20Object%20Reference) (OtherActor :type Actor%20Object%20Reference) (OtherComp :type Primitive%20Component%20Object%20Reference) (OtherBodyIndex :type Integer) (bFromSweep :type Boolean) (SweepResult :type Hit%20Result%20Structure%20%28by%20ref%29))
  (if (== OtherActor (Game|GetPlayerCharacter 0))
    (Game|Damage|ApplyDamage OtherActor 3e+01 0 0)))

(event EventBeginPlay
  (Components|Animation|PlayAnimation (Variables|Default|GetSkeletalMesh) "/Game/Robert/spike_floor_Start.spike_floor_Start" false)
  (if (Variables|Default|GetActivate)
    (Variables|Default|SetCanPlay true)
    (Variables|Default|SetTime_Between%20activate (Math|Random|RandomIntegerinRange 1 7))
    (else
      (Variables|Default|SetCanPlay false))))

(event Collision|EventActorBeginOverlap
  (params (OtherActor :type Actor%20Object%20Reference)))

(event EventTick
  (params (DeltaSeconds :type Float%20%28single-precision%29))
  (if (Variables|Default|GetCanPlay)
    (Components|Animation|PlayAnimation (Variables|Default|GetSkeletalMesh) "/Game/Bowen/spike_floor_Anim.spike_floor_Anim" false)
    (Variables|Default|SetCanPlay false)
    (Utilities|FlowControl|Delay (Math|Conversions|ToFloat(Integer) (Variables|Default|GetTime_Between%20activate)))
    (Variables|Default|SetTime_Between%20activate (Math|Random|RandomIntegerinRange 1 7))
    (Variables|Default|SetCanPlay true)))

(fn ConstructionScript)